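; BP_Enemy is a side-scroller flipbook enemy that patrols along the X axis and can be stomped by BP_Character.
; Tick feeds a signed Velocity into movement input, and either turn box flips its sign when an overlap ends.
; The attack box sets the player's BisDead flag.
; The top box plays a damage sound, launches the player upward and calls Death, which disables collision and movement, swaps the flipbook and expires the actor.
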(event `self.ReceiveTick`
  (params (DeltaSeconds :type "Float (single-precision)"))
  (`self.AddMovementInput` (1.0 0.0 0.0) (`self.Velocity`)))

(event `self.Box_Turn1.OnComponentEndOverlap`
  (params (OverlappedComponent :type "PrimitiveComponent Object Reference") (OtherActor :type "Actor Object Reference") (OtherComp :type "PrimitiveComponent Object Reference") (OtherBodyIndex :type Integer))
  (set `self.Velocity` (* (`self.Velocity`) -1.0) :!label _label))

(event `self.Box_Turn2.OnComponentEndOverlap`
  (params (OverlappedComponent :type "PrimitiveComponent Object Reference") (OtherActor :type "Actor Object Reference") (OtherComp :type "PrimitiveComponent Object Reference") (OtherBodyIndex :type Integer))
  (goto _label))

(event `self.Box_Attack.OnComponentBeginOverlap`
  (params (OverlappedComponent :type "PrimitiveComponent Object Reference") (OtherActor :type "Actor Object Reference") (OtherComp :type "PrimitiveComponent Object Reference") (OtherBodyIndex :type Integer) (bFromSweep :type Boolean) (SweepResult :type "HitResult Structure (by ref)"))
  (bind _asbp_character (cast `/Game/MyContects/BP/BP_Character` OtherActor))
  (set `/Game/MyContects/BP/BP_Character.bisDead` true _asbp_character))

(event `self.Box_Top.OnComponentBeginOverlap`
  (params (OverlappedComponent :type "PrimitiveComponent Object Reference") (OtherActor :type "Actor Object Reference") (OtherComp :type "PrimitiveComponent Object Reference") (OtherBodyIndex :type Integer) (bFromSweep :type Boolean) (SweepResult :type "HitResult Structure (by ref)"))
  (`GameplayStatics.PlaySound2D` "/Game/MyContects/BGM-SE/Damage.Damage" 1.0 1.0 0.0 null null)
  (bind _asbp_character (cast `/Game/MyContects/BP/BP_Character` OtherActor))
  (`self.LaunchCharacter` _asbp_character (0.0 0.0 1000.0) false true)
  (`self.Death`))

(event `Death`
  (`self.SetActorEnableCollision` false)
  (`PaperFlipbookComponent.SetFlipbook` (`self.Sprite`) "/Game/MyContects/Sprite/Enemy/Enemy1_Death.Enemy1_Death")
  (`CharacterMovementComponent.DisableMovement` (`self.CharacterMovement`))
  (`self.SetLifeSpan` 1.0))

(fn `UserConstructionScript`)